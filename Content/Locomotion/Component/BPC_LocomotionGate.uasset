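; Character component that manages locomotion gaits ("gates") and crouch toggling on its owning Character.
; UpdateGate sends the gait to the mesh's AnimInstance by message and, if that returns true, applies movement speed, acceleration and braking values from the GateSetting map.
; BeginPlay sets the initial gait, while IA_Jog switches gait on press and reverts to LastGate on release.
; A raw C key toggles crouch, only crouching when not falling, with debug prints.
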(event `self.ReceiveBeginPlay`
  (`self.Update gate` "NewEnumerator1"))

(event `Key|C`
  (params (Key :type "Key Structure"))
  (bind _returnvalue (`self.GetOwner`))
  (bind _ascharacter (cast `Character` _returnvalue :!pure true))
  (:`Pressed`
    (if (and (not (`Character.bIsCrouched` _ascharacter)) (not (`NavMovementInterface.IsFalling` (`Actor.GetComponentByClass` _returnvalue "/Script/Engine.CharacterMovementComponent"))))
      (`Character.Crouch` _ascharacter)
      (`KismetSystemLibrary.PrintString` "Hello")
      (else
        (`Character.UnCrouch` _ascharacter)
        (`KismetSystemLibrary.PrintString` "by")))))

(event `EnhancedInput|/Game/Input/Actions/IA_Jog`
  (params (ActionValue :type Boolean) (ElapsedSeconds :type "Float (double-precision)") (TriggeredSeconds :type "Float (double-precision)") (InputAction :type "InputAction Object Reference" :default "/Game/Input/Actions/IA_Jog.IA_Jog"))
  (:`Started`
    (`self.Update gate` "NewEnumerator2"))
  (:`Completed`
    (`self.Update gate` (`self.Last Gate`))))

(fn `Get Anim Instance`
  (returns (NewParam :type "AnimInstance Object Reference"))
  (return (`SkeletalMeshComponent.GetAnimInstance` (`Character.Mesh` (cast `Character` (`self.GetOwner`) :!pure true)))))

(fn `Receive Gate Data`
  (params (Gate :type "/Game/Locomotion/Enum/E_Gate Enum" :default "NewEnumerator0"))
  (returns (`Success?` :type Boolean))
  (return false))

(fn `Update gate`
  (params (`Desierd Gate` :type "/Game/Locomotion/Enum/E_Gate Enum" :default "NewEnumerator0"))
  (bind _returnvalue (`Actor.GetComponentByClass` (`self.GetOwner`) "/Script/Engine.CharacterMovementComponent"))
  (bind (_movementspeed _maxacceleration _brakingdeceleration _brakingfrictionfactor _useseperatebrakingfriction _brakingfriction) (break `/Game/Locomotion/Structuer/ST_Locomotio_GateSetting` (`BlueprintMapLibrary.Map_Find` (`self.Gate Setting`) (`local.Desierd Gate`))))
  (set `self.Last Gate` (`self.Current Gate`))
  (set `self.Current Gate` (`local.Desierd Gate`))
  (bind _success_ (message `/Game/Locomotion/Interface/BPI_GateData.Receive Gate Data` (`self.Get Anim Instance`) (`local.Desierd Gate`)))
  (if _success_
    (set `CharacterMovementComponent.MaxWalkSpeed` _movementspeed _returnvalue)
    (set `CharacterMovementComponent.MaxAcceleration` _maxacceleration _returnvalue)
    (set `CharacterMovementComponent.BrakingDecelerationWalking` _brakingdeceleration _returnvalue)
    (set `CharacterMovementComponent.BrakingFrictionFactor` _brakingfrictionfactor _returnvalue)
    (set `CharacterMovementComponent.bUseSeparateBrakingFriction` _useseperatebrakingfriction _returnvalue)
    (set `CharacterMovementComponent.BrakingFriction` _brakingfriction _returnvalue)
    (else
      (`KismetSystemLibrary.PrintString` "Fuckkk"))))